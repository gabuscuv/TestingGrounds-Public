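; Behavior tree task that picks the next patrol waypoint for a patrolling guard NPC.
; It reads the patrol point array from the controlled BP_PatrollingGuard and steps to the entry after the last stored PatrolPoint, wrapping to the first at the end.
; The chosen point is saved on the task and written to the Waypoint blackboard key, then the task finishes successfully.
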(event EventReceiveExecuteAI
  (params (OwnerController :type AI%20Controller%20Object%20Reference) (ControlledPawn :type Pawn%20Object%20Reference))
  (bind _patrols_point (CallFunction|GetPatrolPoints ControlledPawn))
  (bind _actor (CallFunction|NewFunction0 _patrols_point))
  (Class|BTFunctionLibrary|SetBlackboardValueasObject (Variables|Default|GetWaypoint) _actor)
  (AI|BehaviorTree|FinishExecute true))

(fn GetPatrolPoints
  (params (Object :type Object%20Object%20Reference))
  (bind _asbp_patrolling_guard (Utilities|Casting|CastToBP_PatrollingGuard Object))
  (return (Variables|/Game/Dynamic/NPC/_Characters/BP_PatrollingGuard.BP_PatrollingGuard_C|GetPatrolsPoint _asbp_patrolling_guard)))

(fn NewFunction0
  (params (TargetArray :type Array%20of%20Actor%20Object%20References))
  (if (!= (Utilities|Array|FindItem TargetArray (Variables|Default|GetPatrolPoint)) (- (Utilities|Array|Length TargetArray) 1))
    (bind _output_get (Variables|Default|SetPatrolPoint (Utilities|Array|Get(acopy) TargetArray (+ (Utilities|Array|FindItem TargetArray (Variables|Default|GetPatrolPoint)) 1))))
    (return _output_get)
    (else
      (bind _output_get_2 (Variables|Default|SetPatrolPoint (Utilities|Array|Get(acopy) TargetArray)))
      (return _output_get_2))))