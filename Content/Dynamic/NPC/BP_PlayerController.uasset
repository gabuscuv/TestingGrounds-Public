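; Player controller that tracks the score and remaining tries, and can revive the player's original patrolling guard pawn.
; It caches the controlled pawn at BeginPlay, and GetOldPawn casts that reference to BP_PatrollingGuard.
; Revive calls the guard's own Revive and decrements Tries, with no check on how many remain.
; AddScore and GetScore maintain and expose the running score.
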(event EventBeginPlay
  (Variables|Default|SetOldPawn (Pawn|GetControlledPawn)))

(event EventTick
  (params (DeltaSeconds :type Float%20%28single-precision%29)))

(fn ConstructionScript)

(fn GetOldPawn
  (bind _asbp_patrolling_guard (Utilities|Casting|CastToBP_PatrollingGuard (Variables|Default|GetOldPawn)))
  (return _asbp_patrolling_guard))

(fn Revive
  (bind _newparam (CallFunction|GetOldPawn))
  (Default|Revive _newparam)
  (Variables|Default|SetTries (- (Variables|Default|GetTries) 1)))

(fn AddScore
  (params (Points :type Integer))
  (bind _output_get (Variables|Default|SetScore (+ Points (Variables|Default|GetScore))))
  (return _output_get))

(fn GetScore
  (return (Variables|Default|GetScore)))