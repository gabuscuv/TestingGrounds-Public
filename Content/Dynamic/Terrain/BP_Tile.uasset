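; Terrain tile for a chain of spawned tiles that fills itself with random props and, unless flagged empty, patrolling guards scaled by the game mode's enemy multiplier.
; Its barrier starts green and passable, then turns red and solid when the player leaves the first trigger box.
; Entering the second box cleans up child actors, destroys the tile and has the game mode spawn another.
; An arrow component supplies the attach transform.
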(event OnComponentEndOverlap(Box)
  (params (OverlappedComponent :type Primitive%20Component%20Object%20Reference) (OtherActor :type Actor%20Object%20Reference) (OtherComp :type Primitive%20Component%20Object%20Reference) (OtherBodyIndex :type Integer))
  (Utilities|IsPlayer OtherActor)
  (CallFunction|Lock (Variables|Default|GetStaticMesh)))

(event OnComponentBeginOverlap(Box1)
  (params (OverlappedComponent :type Primitive%20Component%20Object%20Reference) (OtherActor :type Actor%20Object%20Reference) (OtherComp :type Primitive%20Component%20Object%20Reference) (OtherBodyIndex :type Integer) (bFromSweep :type Boolean) (SweepResult :type Hit%20Result%20Structure%20%28by%20ref%29))
  (Utilities|IsPlayer OtherActor)
  (Class|ActorGarbageCollector|CleanParentActors (Variables|Default|GetActorGarbageCollector))
  (Actor|DestroyActor)
  (bind _asbp_game_mode_main (Utilities|Casting|CastToBP_GameModeMain (Game|GetGameMode)))
  (Default|SpawnNewTile _asbp_game_mode_main))

(event EventBeginPlay
  (CallFunction|SpawnRandomActors)
  (CallFunction|Unlock (Variables|Default|GetStaticMesh)))

(fn ConstructionScript)

(fn GetAttachLocation
  (return (Transformation|GetWorldTransform (Variables|Default|GetArrow))))

(fn ChangeBarrierStatus
  (params (Barrier :type Static%20Mesh%20Component%20Object%20Reference) (CollisionStatus :type ECollisionEnabled%20Enum :default "NoCollision") (MaterialToSet :type Material%20Interface%20Object%20Reference))
  (Collision|SetCollisionEnabled Barrier CollisionStatus)
  (Rendering|Material|SetMaterial Barrier 0 MaterialToSet)
  (return))

(fn Unlock
  (params (NewParam :type Static%20Mesh%20Component%20Object%20Reference))
  (CallFunction|ChangeBarrierStatus NewParam "NoCollision" "/Game/Dynamic/Terrain/M_GreenBarrier.M_GreenBarrier")
  (return))

(fn Lock
  (params (NewParam :type Static%20Mesh%20Component%20Object%20Reference))
  (CallFunction|ChangeBarrierStatus NewParam "QueryAndPhysics" "/Game/Dynamic/Terrain/M_RedBarrier.M_RedBarrier")
  (return))

(fn SpawnRandomActors
  (for _array_element (Variables|Default|GetItemsTypeRef)
    (Class|Tile|PlaceActors _array_element 1 3 1e+03 1.0 3.0))
  (if (not (Variables|Default|GetIsEmpty))
    (bind _asbp_game_mode_main (Utilities|Casting|CastToBP_GameModeMain (Game|GetGameMode)))
    (bind (_minspawn _maxspawn) (Default|GetEnemyMultiplier _asbp_game_mode_main))
    (Class|Tile|PlaceAIPawns "/Game/Dynamic/NPC/_Characters/BP_PatrollingGuard.BP_PatrollingGuard_C" _minspawn _maxspawn 5e+02)))