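; BP_ItemGeneric is a generic pickup item that spins in place and destroys itself when the player overlaps it.
; IsPlayerOverlapping identifies the player by casting the overlapping actor to BP_PatrollingGuard, despite that class's name, and also returns the cast reference.
; Tick adds a fixed rotation to the Scene component each frame, so spin speed depends on frame rate.
; A note on the overlap check points to inherited items, suggesting this serves as their parent class.
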(event EventBeginPlay)

(event Collision|EventActorBeginOverlap
  (params (OtherActor :type Actor%20Object%20Reference))
  (bind _isplayer (CallFunction|IsPlayerOverlapping OtherActor))
  (if _isplayer
    (Actor|DestroyActor)))

(event EventTick
  (params (DeltaSeconds :type Float%20%28single-precision%29))
  (bind _scene (Variables|Default|GetScene))
  (Transformation|SetRelativeRotation _scene (Math|Rotator|CombineRotators (Variables|/Script/Engine.SceneComponent|GetRelativeRotation _scene) "0.000000,1.000000,0.000000") false false))

(fn ConstructionScript)

(fn IsPlayerOverlapping
  (params (Object :type Object%20Object%20Reference))
  ;[1 1 1] Check inherited Items (No references in parent class)
  (bind _asbp_patrolling_guard (Utilities|Casting|CastToBP_PatrollingGuard Object)
    (:then
      (return true _asbp_patrolling_guard))
    (:CastFailed
      (return false 0))))