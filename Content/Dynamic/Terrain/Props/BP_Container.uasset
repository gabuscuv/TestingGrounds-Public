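; Container prop that supplies a random pickup, either a potion or ammo, when play begins.
; A Spawn helper creates the chosen actor using the Arrow component's relative transform, then attaches it with KeepRelative rules so that offset becomes local to the container.
; On EndPlay, the ActorGarbageCollector component runs its CleanParentActors cleanup.
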(event EventBeginPlay
  (if (Math|Random|RandomBool)
    (CallFunction|Spawn "/Game/Dynamic/Terrain/Props/BP_Potion.BP_Potion_C")
    (else
      (CallFunction|Spawn "/Game/Dynamic/Terrain/Props/BP_Ammo.BP_Ammo_C"))))

(event Collision|EventActorBeginOverlap
  (params (OtherActor :type Actor%20Object%20Reference)))

(event EventTick
  (params (DeltaSeconds :type Float%20%28single-precision%29)))

(event EventEndPlay
  (params (EndPlayReason :type EEndPlayReason%20Enum :default "Destroyed"))
  (Class|ActorGarbageCollector|CleanParentActors (Variables|Default|GetActorGarbageCollector)))

(fn ConstructionScript)

(fn Spawn
  (params (Ac :type Actor%20Class%20Reference))
  (bind _returnvalue (Game|SpawnActorfromClass Ac (Transformation|GetRelativeTransform (Variables|Default|GetArrow)) "Undefined" 0 0))
  (Utilities|IsValid _returnvalue
    (:Is%20Valid
      (Transformation|AttachActorToActor _returnvalue self "None" "KeepRelative" "KeepRelative" "KeepRelative" true))))