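; BP_Potion is a health pickup prop that heals the player on contact.
; On actor overlap it uses IsPlayerOverlapping to filter for the player, then RecoverHealth adds HealthToSum to that player's Health with no clamping in this Blueprint.
; The parent class's overlap handler runs only after a successful heal, so non-player overlaps never reach it.
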(event EventBeginPlay
  (|CallParentFunction) ; This node is disabled and will not be called.\nDrag off pins to build functionality.
)

(event Collision|EventActorBeginOverlap
  (params (OtherActor :type Actor%20Object%20Reference))
  (bind (_isplayer _player) (CallFunction|IsPlayerOverlapping OtherActor))
  (if _isplayer
    (CallFunction|RecoverHealth _player)
    (|CallParentFunction OtherActor)))

(event EventTick
  (params (DeltaSeconds :type Float%20%28single-precision%29))
  (|CallParentFunction DeltaSeconds) ; This node is disabled and will not be called.\nDrag off pins to build functionality.
)

(fn ConstructionScript
  (|CallParentFunction))

(fn RecoverHealth
  (params (PatrollingGuard :type BP%20Patrolling%20Guard%20Object%20Reference))
  (Variables|/Game/Dynamic/NPC/_Characters/BP_PatrollingGuard.BP_PatrollingGuard_C|SetHealth PatrollingGuard (+ (Variables|/Game/Dynamic/NPC/_Characters/BP_PatrollingGuard.BP_PatrollingGuard_C|GetHealth PatrollingGuard) (Variables|Default|GetHealthToSum))))