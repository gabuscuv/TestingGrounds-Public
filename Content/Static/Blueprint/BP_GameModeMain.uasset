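; Main game mode for an endless tile-based level: spawns tiles, awards conquest points, handles pause and shows a first-time tutorial.
; Random tile types chain via each tile's attach location up to a cap, and each receives a pool of nav mesh bounds volumes.
; Conquests add to the player controller's score, updating a high score SaveGame loaded on BeginPlay and saved on EndPlay.
; Enemy spawn ranges scale with score.
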(event EventBeginPlay
  (Utilities|FlowControl|Sequence
    (:then_0
      (if (not (Class|KismetSystemLibrary|IsPackagedforDistribution))
        (CallFunction|DebugConsole (Game|GetPlayerController 0))))
    (:then_1
      (CallFunction|LoadHighScore)
      (if (Variables|Default|GetbFirstTime)
        (CallFunction|ShowTutorial (Game|GetPlayerController 0)))
      (Class|GameModeMain|PopulateBoundsVolumePool)
      (CallFunction|SpawnTile)
      (CallFunction|NewTileConquered))))

(event EventTick
  (params (DeltaSeconds :type Float%20%28single-precision%29)))

(event EventEndPlay
  (params (EndPlayReason :type EEndPlayReason%20Enum :default "Destroyed"))
  (CallFunction|SaveHighScore))

(event Input|ActionEvents|InputActionPause
  (params (Key :type Key%20Structure))
  (:Released
    (Game|SetGamePaused (not (Game|IsGamePaused)))))

(fn ConstructionScript)

(fn SpawnTile
  (bind _tilestypesarray (Variables|Default|GetTilesTypesArray))
  (for _index (range (Class|GameModeMain|TileCount) (Variables|Spawns|GetMaxTilesSpawn))
    (bind _returnvalue (Game|SpawnActorfromClass (Utilities|Array|Get(acopy) _tilestypesarray (Math|Random|RandomInteger (Utilities|Array|Length _tilestypesarray))) (Variables|Default|GetNextTileTransform) "Undefined" 0 0))
    (bind _newparam (Default|GetAttachLocation _returnvalue))
    (Variables|Default|SetNextTileTransform _newparam)
    (Class|Tile|SetPool _returnvalue (Variables|Default|GetNavMeshBoundsVolume))))

(fn SpawnNewTile
  (CallFunction|SpawnTile)
  (Class|GameModeMain|PopulateBoundsVolumePool)
  (CallFunction|NewTileConquered))

(fn NewTileConquered
  (bind _asbp_player_controller (Utilities|Casting|CastToBP_PlayerController (Game|GetPlayerController 0)))
  (bind _currentpoints (Default|AddScore _asbp_player_controller (Variables|Points|GetPointsByConquest)))
  (if (> _currentpoints (Variables|/Game/Dynamic/Blueprints/HighScore.HighScore_C|GetScore (Variables|Default|GetHighScore)))
    (Default|SetHighScore (Variables|Default|GetHighScore) _currentpoints)))

(fn SaveHighScore
  (bind _returnvalue (SaveGame|SaveGametoSlot (Variables|Default|GetHighScore) (Variables|Default|GetHighScoreFilename)))
  (if _returnvalue
    (Development|PrintString "Saved High Score")
    (else
      (Development|PrintString "Failed High Score")))
  (return))

(fn LoadHighScore
  (bind _highscorefilename (Variables|Default|GetHighScoreFilename))
  (bind _returnvalue (SaveGame|DoesSaveGameExist _highscorefilename))
  (if _returnvalue
    (bind _returnvalue_2 (SaveGame|LoadGamefromSlot _highscorefilename))
    (bind _ashigh_score (Utilities|Casting|CastToHighScore _returnvalue_2)
      (:then
        (Variables|Default|SetHighScore _ashigh_score)
        (Variables|Default|SetbFirstTime false))
      (:CastFailed
        (bind _returnvalue_3 (SaveGame|CreateSaveGameObject "/Game/Dynamic/Blueprints/HighScore.HighScore_C" :!label _label))
        (Variables|Default|SetHighScore _returnvalue_3)))
    (else
      (goto _label)))
  (return))

(fn GetHighScore
  (bind _score (Default|GetHighScore (Variables|Default|GetHighScore)))
  (return _score))

(fn GetEnemyMultiplier
  (bind _returnvalue (Class|KismetSystemLibrary|MakeLiteralInteger 1))
  (bind _maxmultiplier (Variables|Spawns|GetMaxMultiplier))
  (bind _maxenemiesbytile (Variables|Spawns|GetMaxEnemiesByTile))
  (bind _asbp_player_controller (Utilities|Casting|CastToBP_PlayerController (Game|GetPlayerController 0)))
  (if (== (/ (Default|GetScore _asbp_player_controller) 10) 0)
    (return _returnvalue _returnvalue)
    (elif (!= (/ (Default|GetScore _asbp_player_controller) 10) _maxmultiplier)
      (return (* (Variables|Spawns|GetMinEnemiesByTile) (/ (Default|GetScore _asbp_player_controller) 10)) (* (Variables|Spawns|GetMaxEnemiesByTile) (/ (Default|GetScore _asbp_player_controller) 10)))
      (else
        (return (* _maxenemiesbytile _maxmultiplier) (* _maxenemiesbytile _maxmultiplier))))))

(fn DebugConsole
  (params (SpecificPlayer :type Player%20Controller%20Object%20Reference))
  (Utilities|FlowControl|Sequence
    (:then_0
      (Development|ExecuteConsoleCommand "Stat UnitGraph" SpecificPlayer))))

(fn ShowTutorial
  (params (PlayerController :type Player%20Controller%20Object%20Reference))
  (Game|SetGamePaused true)
  (bind _returnvalue (UserInterface|CreateWidget "/Game/Dynamic/UI/WBP_Tutorial.WBP_Tutorial_C" 0 0))
  (UserInterface|Viewport|AddtoPlayerScreen _returnvalue)
  (Input|SetInputModeUIOnly PlayerController _returnvalue "DoNotLock"))